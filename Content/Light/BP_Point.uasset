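; BP_Point is a point light actor that reports how strongly it illuminates the player character.
; It caches the player character on BeginPlay.
; When CE_Illuminated is called, it checks the light's attenuation radius, then line-traces to the character, ignoring the passed IBear actor, to confirm nothing blocks it.
; On a hit it sends the character the light's intensity, scaled down linearly with distance.
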(event Custom|CE_Illuminated
  (params (I_Bear :type BP%20Bear%20Object%20Reference))
  (if (<= (Math|Vector|Distance(Vector) (Transformation|GetActorLocation) (Transformation|GetActorLocation (Variables|Default|GetV_Character))) (Variables|/Script/Engine.LocalLightComponent|GetAttenuationRadius (Variables|Default|GetLight)))
    (bind _outhit (Collision|LineTraceForObjects (Transformation|GetActorLocation) (Transformation|GetActorLocation (Variables|Default|GetV_Character)) (Utilities|Array|MakeArray "ObjectTypeQuery1" "ObjectTypeQuery2" "ObjectTypeQuery3" "ObjectTypeQuery4" "ObjectTypeQuery5" "ObjectTypeQuery6") false (Utilities|Array|MakeArray I_Bear) "None"))
    (Utilities|Casting|CastToBP_ThirdPersonCharacter (.hitactor _outhit))
    (Default|CEIlluminated (Variables|Default|GetV_Character) (* (Variables|/Script/Engine.LightComponentBase|GetIntensity (Variables|Default|GetLight)) (- 1.0 (/ (Math|Vector|Distance(Vector) (Transformation|GetActorLocation) (Transformation|GetActorLocation (Variables|Default|GetV_Character))) (Variables|/Script/Engine.LocalLightComponent|GetAttenuationRadius (Variables|Default|GetLight))))))))

(event EventBeginPlay
  (bind _asbp_third_person_character (Utilities|Casting|CastToBP_ThirdPersonCharacter (Game|Player|GetPlayerPawn 0)))
  (Variables|Default|SetV_Character _asbp_third_person_character))

(fn ConstructionScript)