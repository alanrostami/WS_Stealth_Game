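; BP_Light is a light actor that tracks whether BP_ThirdPersonCharacter is inside its range.
; BeginPlay caches the player and seeds an overlap flag with a sphere query on Collision, which begin and end overlap events then update.
; Tick traces from the light to the character and casts the hit actor, but nothing follows.
; A disconnected branch would pass intensity, scaled by distance relative to attenuation radius, to CEIlluminated.
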(event EventTick
  (params (DeltaSeconds :type Float%20%28single-precision%29))
  (bind _outhit (Collision|LineTraceForObjects (Transformation|GetActorLocation) (Transformation|GetActorLocation (Variables|Default|GetV_Character)) (Utilities|Array|MakeArray "ObjectTypeQuery1" "ObjectTypeQuery2" "ObjectTypeQuery3" "ObjectTypeQuery4" "ObjectTypeQuery5" "ObjectTypeQuery6") false 0 "None"))
  (Utilities|Casting|CastToBP_ThirdPersonCharacter (.hitactor _outhit)))

(event EventBeginPlay
  (bind _asbp_third_person_character (Utilities|Casting|CastToBP_ThirdPersonCharacter (Game|Player|GetPlayerPawn 0)))
  (Variables|Default|SetV_Character _asbp_third_person_character)
  (bind _returnvalue (Collision|SphereOverlapActors (Transformation|GetWorldLocation (Variables|Default|GetCollision)) (Components|Sphere|GetScaledSphereRadius (Variables|Default|GetCollision)) (Utilities|Array|MakeArray "ObjectTypeQuery3") "/Game/ThirdPerson/Blueprints/BP_ThirdPersonCharacter.BP_ThirdPersonCharacter_C"))
  (Variables|Default|SetV_Overlapped _returnvalue))

(event Collision|EventActorBeginOverlap
  (params (OtherActor :type Actor%20Object%20Reference))
  (Utilities|Casting|CastToBP_ThirdPersonCharacter OtherActor)
  (Variables|Default|SetV_Overlapped true))

(event Collision|EventActorEndOverlap
  (params (OtherActor :type Actor%20Object%20Reference))
  (Utilities|Casting|CastToBP_ThirdPersonCharacter OtherActor)
  (Variables|Default|SetV_Overlapped false))

(fn ConstructionScript)