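; Directional light actor, such as a sun, that tells the player character how strongly it is lit.
; On CE_Illuminated, while the light is not pointing upward, it traces from far back along the light direction to the cached player, ignoring the passed-in IBear actor.
; An unblocked trace calls CEIlluminated on the player with light intensity scaled by the downward angle and a constant multiplier.
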(event Custom|CE_Illuminated
  (params (I_Bear :type BP%20Bear%20Object%20Reference))
  (if (<= (.z (Math|Vector|GetForwardVector (Transformation|GetActorRotation))) 0.0)
    (bind _outhit (Collision|LineTraceForObjects (- (Transformation|GetActorLocation (Variables|Default|GetV_Character)) (* (Math|Vector|GetForwardVector (Transformation|GetActorRotation)) 999999999.0)) (Transformation|GetActorLocation (Variables|Default|GetV_Character)) (Utilities|Array|MakeArray "ObjectTypeQuery1" "ObjectTypeQuery2" "ObjectTypeQuery3" "ObjectTypeQuery4" "ObjectTypeQuery5" "ObjectTypeQuery6") false (Utilities|Array|MakeArray I_Bear) "None"))
    (Utilities|Casting|CastToBP_ThirdPersonCharacter (.hitactor _outhit))
    (Default|CEIlluminated (Variables|Default|GetV_Character) (* (* (Variables|/Script/Engine.LightComponentBase|GetIntensity (Variables|Default|GetLight)) (* (.z (Math|Vector|GetForwardVector (Transformation|GetActorRotation))) -1.0)) 1e+03))))

(event EventBeginPlay
  (bind _asbp_third_person_character (Utilities|Casting|CastToBP_ThirdPersonCharacter (Game|Player|GetPlayerPawn 0)))
  (Variables|Default|SetV_Character _asbp_third_person_character))

(fn ConstructionScript)