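; BP_Spot is a spot light that reports to the player's BP_ThirdPersonCharacter how strongly it illuminates them.
; When CE_Illuminated is called with a bear, it checks the player is within attenuation radius and at an angle between the inner and outer cones.
; A line trace ignoring that bear must hit the player.
; It then calls CEIlluminated on the character with intensity scaled by linear distance falloff.
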(event Custom|CE_Illuminated
  (params (I_Bear :type BP%20Bear%20Object%20Reference))
  (Variables|Default|SetV_Bear I_Bear)
  (if (<= (Math|Vector|Distance(Vector) (Transformation|GetActorLocation) (Transformation|GetActorLocation (Variables|Default|GetV_Character))) (Variables|/Script/Engine.LocalLightComponent|GetAttenuationRadius (Variables|Default|GetLight)))
    (if (Math|Float|InRange(Float) (Class|KismetMathLibrary|DegAcos (Math|Vector|DotProduct (Math|Vector|Normalize (- (Transformation|GetActorLocation (Variables|Default|GetV_Character)) (Transformation|GetActorLocation))) (Transformation|GetActorForwardVector))) (Variables|/Script/Engine.SpotLightComponent|GetInnerConeAngle (Variables|Default|GetLight)) (Variables|/Script/Engine.SpotLightComponent|GetOuterConeAngle (Variables|Default|GetLight)))
      (bind _outhit (Collision|LineTraceForObjects (Transformation|GetActorLocation) (Transformation|GetActorLocation (Variables|Default|GetV_Character)) (Utilities|Array|MakeArray "ObjectTypeQuery1" "ObjectTypeQuery2" "ObjectTypeQuery3" "ObjectTypeQuery4" "ObjectTypeQuery5" "ObjectTypeQuery6") false (Utilities|Array|MakeArray (Variables|Default|GetV_Bear)) "None"))
      (Utilities|Casting|CastToBP_ThirdPersonCharacter (.hitactor _outhit))
      (Default|CEIlluminated (Variables|Default|GetV_Character) (* (Variables|/Script/Engine.LightComponentBase|GetIntensity (Variables|Default|GetLight)) (- 1.0 (/ (Math|Vector|Distance(Vector) (Transformation|GetActorLocation) (Transformation|GetActorLocation (Variables|Default|GetV_Character))) (Variables|/Script/Engine.LocalLightComponent|GetAttenuationRadius (Variables|Default|GetLight)))))))))

(event EventBeginPlay
  (bind _asbp_third_person_character (Utilities|Casting|CastToBP_ThirdPersonCharacter (Game|Player|GetPlayerPawn 0)))
  (Variables|Default|SetV_Character _asbp_third_person_character))

(fn ConstructionScript)