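; BP_Bear is a throwable bear actor linked to the player's third-person character.
; CE_Thrown stores a direction, resets the timer and activates an effect, then Tick offsets the actor at constant speed.
; A line trace ahead, ignoring the character, skips movement on frames where it would hit something.
; Once the flight duration elapses, it clears the thrown state and calls CEReturned on the character, which handles any return.
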(event Custom|CE_Returned
  (Variables|Default|SetV_Thrown false)
  (Default|CEReturned (Variables|Default|GetV_Character)))

(event Custom|CE_Thrown
  (params (I_Forward :type Vector))
  (Variables|Default|SetV_Thrown true)
  (Variables|Default|SetV_Forward I_Forward)
  (Variables|Default|SetV_Timer 0.0)
  (Components|Activation|Activate (Variables|Default|GetEffect) false))

(event EventBeginPlay
  (bind _asbp_third_person_character (Utilities|Casting|CastToBP_ThirdPersonCharacter (Game|Player|GetPlayerPawn 0)))
  (Variables|Default|SetV_Character _asbp_third_person_character))

(event EventTick
  (params (DeltaSeconds :type Float%20%28single-precision%29))
  (Variables|Default|SetV_Delta DeltaSeconds)
  (if (Variables|Default|GetV_Thrown)
    (Variables|Default|SetV_Timer (+ (Variables|Default|GetV_Delta) (Variables|Default|GetV_Timer)))
    (if (< (+ (Variables|Default|GetV_Delta) (Variables|Default|GetV_Timer)) (Variables|Default|GetC_Duration))
      (bind _returnvalue (Collision|LineTraceForObjects (Transformation|GetActorLocation) (+ (Transformation|GetActorLocation) (* (* (Variables|Default|GetV_Delta) (Variables|Default|GetV_Forward)) (Variables|Default|GetC_Speed))) (Utilities|Array|MakeArray "ObjectTypeQuery1" "ObjectTypeQuery2" "ObjectTypeQuery3" "ObjectTypeQuery4" "ObjectTypeQuery5" "ObjectTypeQuery6") false (Utilities|Array|MakeArray (Variables|Default|GetV_Character)) "None"))
      (if (not _returnvalue)
        (Transformation|AddActorWorldOffset (* (* (Variables|Default|GetV_Delta) (Variables|Default|GetV_Forward)) (Variables|Default|GetC_Speed))))
      (else
        (CallFunction|CEReturned)))))

(fn ConstructionScript)