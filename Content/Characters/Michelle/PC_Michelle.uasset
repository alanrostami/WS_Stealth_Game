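; Player controller for the Michelle character that turns Enhanced Input actions into walking, camera look and crouching.
; BeginPlay adds the input mapping context and limits camera pitch.
; Walk input pushes the pawn along control-rotation forward and right vectors at fixed scale, ignoring the action value.
; Crouch calls rely on a BP_Michelle cast that is never executed, and the Roll section is empty.
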(event Input|EnhancedActionEvents|EnhancedInputActionIA_Michelle_Walk
  (params (ActionValue :type Vector%202D%20Structure) (ElapsedSeconds :type Float%20%28double-precision%29) (TriggeredSeconds :type Float%20%28double-precision%29) (InputAction :type Input%20Action%20Object%20Reference :default "/Game/Characters/Michelle/Input/IA_Michelle_Walk.IA_Michelle_Walk"))
  (bind _returnvalue (Pawn|GetControlledPawn))
  (bind _returnvalue_2 (Pawn|GetControlRotation :!class /Script/Engine.Controller))
  (:Triggered
    (Pawn|Input|AddMovementInput _returnvalue (Math|Vector|GetForwardVector _returnvalue_2) 1.0 false)
    (Pawn|Input|AddMovementInput _returnvalue (Math|Vector|GetRightVector _returnvalue_2) 1.0 false)))

(event Input|EnhancedActionEvents|EnhancedInputActionIA_Camera
  (params (ActionValue :type Vector%202D%20Structure) (ElapsedSeconds :type Float%20%28double-precision%29) (TriggeredSeconds :type Float%20%28double-precision%29) (InputAction :type Input%20Action%20Object%20Reference :default "/Game/Characters/Michelle/Input/IA_Camera.IA_Camera"))
  (:Triggered
    (Class|PlayerController|AddYawInput (.x ActionValue))
    (Class|PlayerController|AddPitchInput (.y ActionValue))))

(event Input|EnhancedActionEvents|EnhancedInputActionIA_Michelle_Crouch
  (params (ActionValue :type Vector%202D%20Structure) (ElapsedSeconds :type Float%20%28double-precision%29) (TriggeredSeconds :type Float%20%28double-precision%29) (InputAction :type Input%20Action%20Object%20Reference :default "/Game/Characters/Michelle/Input/IA_Michelle_Crouch.IA_Michelle_Crouch"))
  (:Triggered
    (Character|Crouch (stale _asbp_michelle)))
  (:Completed
    (Character|UnCrouch (stale _asbp_michelle))))

(event Input|EnhancedActionEvents|EnhancedInputActionIA_Michelle_Roll
  (params (ActionValue :type Boolean) (ElapsedSeconds :type Float%20%28double-precision%29) (TriggeredSeconds :type Float%20%28double-precision%29) (InputAction :type Input%20Action%20Object%20Reference :default "/Game/Characters/Michelle/Input/IA_Michelle_Roll.IA_Michelle_Roll")))

(event EventBeginPlay
  (bind _playercameramanager (Variables|Default|GetPlayerCameraManager))
  (Input|AddMappingContext (PlayerController|LocalPlayerSubsystems|GetEnhancedInputLocalPlayerSubsystem 0) 0 0 "(bIgnoreAllPressedKeysUntilRelease=True,bForceImmediately=False)")
  (Variables|/Script/Engine.PlayerCameraManager|SetViewPitchMin _playercameramanager -45.0)
  (Variables|/Script/Engine.PlayerCameraManager|SetViewPitchMax _playercameramanager 35.0))

(fn ConstructionScript)