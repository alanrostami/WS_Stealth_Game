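; Player controller for the protagonist, Michelle, handling Enhanced Input walking and camera pitch limits.
; On BeginPlay it adds the Michelle mapping context and clamps how far the camera can look up and down.
; The walk action moves the controlled pawn along the control rotation's forward (X) and right (Y) vectors, using the full rotation rather than yaw alone.
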(event Input|EnhancedActionEvents|EnhancedInputActionIA_Michelle_Walk
  (params (ActionValue :type Vector%202D%20Structure) (ElapsedSeconds :type Float%20%28double-precision%29) (TriggeredSeconds :type Float%20%28double-precision%29) (InputAction :type Input%20Action%20Object%20Reference :default "/Game/_GameManager/Input/IA_Michelle_Walk.IA_Michelle_Walk"))
  (bind _returnvalue (Pawn|GetControlledPawn))
  (bind _returnvalue_2 (Pawn|GetControlRotation :!class /Script/Engine.Controller))
  (:Triggered
    (Pawn|Input|AddMovementInput _returnvalue (Math|Vector|GetForwardVector _returnvalue_2) (.x ActionValue) false)
    (Pawn|Input|AddMovementInput _returnvalue (Math|Vector|GetRightVector _returnvalue_2) (.y ActionValue) false)))

(event EventBeginPlay
  (bind _playercameramanager (Variables|Default|GetPlayerCameraManager))
  (Input|AddMappingContext (PlayerController|LocalPlayerSubsystems|GetEnhancedInputLocalPlayerSubsystem 0) "/Game/_GameManager/Input/IMC_Michelle.IMC_Michelle" 0 "(bIgnoreAllPressedKeysUntilRelease=True,bForceImmediately=False)")
  (Variables|/Script/Engine.PlayerCameraManager|SetViewPitchMin _playercameramanager -45.0)
  (Variables|/Script/Engine.PlayerCameraManager|SetViewPitchMax _playercameramanager 35.0))

(fn ConstructionScript)